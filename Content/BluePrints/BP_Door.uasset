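; BP_Door is a key-gated door that opens when a player character carrying more than two keys enters its trigger box.
; The box overlap checks KeyAmount on BP_ThirdPersonCharacter, then plays the DOORDOWN timeline, which drives the door mesh's relative Z to lower it.
; With too few keys it shows the Locked component instead, which is hidden whenever an overlap with the box ends.
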(event `self.Box.OnComponentBeginOverlap`
  (params (OverlappedComponent :type "PrimitiveComponent Object Reference") (OtherActor :type "Actor Object Reference") (OtherComp :type "PrimitiveComponent Object Reference") (OtherBodyIndex :type Integer) (bFromSweep :type Boolean) (SweepResult :type "HitResult Structure (by ref)"))
  (bind _door (`self.Door`))
  (bind (_relativelocation_x _relativelocation_y) (`KismetMathLibrary.BreakVector` (`SceneComponent.RelativeLocation` _door)))
  (bind _asbp_third_person_character (cast `/Game/ThirdPerson/Blueprints/BP_ThirdPersonCharacter` OtherActor))
  (if (> (`/Game/ThirdPerson/Blueprints/BP_ThirdPersonCharacter.KeyAmount` _asbp_third_person_character) 2)
    (bind (_direction _lowerdoor) (`Timeline|dOORDOWN`)
      (:`Update`
        (`SceneComponent.K2_SetRelativeLocation` _door (`KismetMathLibrary.MakeVector` _relativelocation_x _relativelocation_y _lowerdoor) false false)))
    (else
      (`SceneComponent.SetVisibility` (`self.Locked`) true false))))

(event `self.Box.OnComponentEndOverlap`
  (params (OverlappedComponent :type "PrimitiveComponent Object Reference") (OtherActor :type "Actor Object Reference") (OtherComp :type "PrimitiveComponent Object Reference") (OtherBodyIndex :type Integer))
  (`SceneComponent.SetVisibility` (`self.Locked`) false false))

(fn `UserConstructionScript`)