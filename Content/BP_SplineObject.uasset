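; BP_SplineObject is an actor that moves along a referenced spline, starting at BeginPlay.
; MoveObject sets the timeline play rate to the inverse of TimeToComplete, then plays it.
; Each timeline update maps the MoveTrack alpha to a distance along the spline's length, then sets the actor's world location and rotation from the spline at that point.
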(event `self.ReceiveBeginPlay`
  (`self.Move Object`))

(event `Move Object`
  (bind _spline (`/Game/BP_SplinPath.Spline` (`self.Spline to follow`)))
  (`TimelineComponent.SetPlayRate` (`self.Time_move`) (/ 1.0 (`self.TimeToComplete`)))
  (bind (_direction _move_track) (`Timeline|Time_move`)
    (:`Update`
      (bind _returnvalue (`KismetMathLibrary.Lerp` 0.0 (`SplineComponent.GetSplineLength` _spline) _move_track))
      (`self.K2_SetActorLocationAndRotation` (`SplineComponent.GetLocationAtDistanceAlongSpline` _spline _returnvalue "World") (`SplineComponent.GetRotationAtDistanceAlongSpline` _spline _returnvalue "World")))))

(fn `UserConstructionScript`)